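; Manager that divides a snow field into a grid of MySnowActorBP areas, spawned through a delayed loop to avoid Blueprint's infinite-loop limit.
; All areas stay active during a timed initialization, then character and shovel colliders attach and only keys around the player's cell are activated each tick.
; Helper functions swap areas between instanced-mesh particles and heightmap-based procedural mesh sections, with G and L keys testing mesh creation and removal.
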(event `SpawnSnowActors`
  ;[1 1 1] SnowActor들 스폰(for loop로 다돌면 언리얼 bp한계로 infinite loop걸려서 다른 구현으로 변경)
  (if (not (and (== (`self.CurrentVerticalIndex`) (- (`self.NumVerticalArea`) 1)) (== (`self.CurrentHorizontalIndex`) (- (`self.NumHorizontalArea`) 1)))) :!label _label
    (`self.SpawnSnowActor` (`self.CurrentVerticalIndex`) (`self.CurrentHorizontalIndex`))
    (if (== (`self.CurrentHorizontalIndex`) (- (`self.NumHorizontalArea`) 1))
      (set `self.CurrentHorizontalIndex` 0)
      (set `self.CurrentVerticalIndex` (+ (`self.CurrentVerticalIndex`) 1))
      (`KismetSystemLibrary.Delay` 0.001)
      (goto _label)
      (else
        (set `self.CurrentHorizontalIndex` (+ (`self.CurrentHorizontalIndex`) 1))
        (`KismetSystemLibrary.Delay` 0.001)
        (goto _label)))
    (else
      (`self.SpawnSnowActor` (`self.CurrentVerticalIndex`) (`self.CurrentHorizontalIndex`)))))

(event `self.ReceiveBeginPlay`
  (`self.EnableInput` (`GameplayStatics.GetPlayerController` 0))
  (`self.InitAreaManager`)
  (`self.SpawnSnowActors`))

(event `Key|G`
  (params (Key :type "Key Structure"))
  (bind _output (`|GetArrayItem` (`self.m_snowActors`) (`self.numClicked`)))
  ;[1 1 1] HeightMap기반 Mesh 생성,제거 테스트코드
  (:`Pressed`
    (if (< (`self.numClicked`) (* (`self.m_numHorizonArea`) (`self.m_numVerticalArea`)))
      (bind _returnvalue (`SnowActorCpp.GetXPos` _output))
      (bind _returnvalue_2 (`SnowActorCpp.GetYPos` _output))
      (bind _returnvalue_3 (`SnowActorCpp.GetZPos` _output))
      (`self.UpdateHeightmap` _returnvalue _returnvalue_2 _returnvalue_3 (`self.numClicked`))
      (`self.MakeMesh` (`self.numClicked`))
      (bind _asmy_snow_actor_bp (cast `/Game/BP/MySnowActorBP` _output))
      (`SceneComponent.SetVisibility` (`/Game/BP/MySnowActorBP.InstancedStaticMesh` _asmy_snow_actor_bp) false false)
      (set `self.numClicked` (+ (`self.numClicked`) 1)))))

(event `Key|L`
  (params (Key :type "Key Structure"))
  ;[1 1 1] HeightMap기반 Mesh 생성,제거 테스트코드
  (:`Pressed`
    (if (> (`self.numClicked`) 0)
      (bind _output_get (set `self.numClicked` (- (`self.numClicked`) 1)))
      (`self.DeleteMesh` _output_get))))

(event `self.ReceiveTick`
  (params (DeltaSeconds :type "Float (single-precision)"))
  ;[1 1 1] Initializing Time Limit이 될때까지는 모든 영역을 활성화/ Time Limit이 끝나면 character collider적용
  (if (`self.IsInitializing`)
    (`self.ActivateAllAreas`)
    (bind _output_get (set `self.AccumulatedDeltaTime` (+ DeltaSeconds (`self.AccumulatedDeltaTime`))))
    (if (>= _output_get (`self.InitializingTimeLimit`))
      (set `self.IsInitializing` false)
      (`self.AttachCharacterColliderToAllSnowActors`)
      (`KismetSystemLibrary.PrintString` "Initializing/character collider적용 완료!")
      (for _array_element (`self.m_snowActors`)
        (bind _asmy_snow_actor_bp (cast `/Game/BP/MySnowActorBP` _array_element))
        (set `/Game/BP/MySnowActorBP.IsSimulating` false _asmy_snow_actor_bp)))
    (else
      ;[1 1 1] 매 프레임 플레이어가 있는 위치기반 활성화되는 snowactor key업데이트
      (bind _returnvalue (`self.GetAreaKey` (`self.K2_GetActorLocation` (`GameplayStatics.GetPlayerCharacter` 0))))
      (`self.ActivateAreas` _returnvalue))))

(fn `ActivateAllAreas`
  (`KismetArrayLibrary.Array_Clear` (`self.ActivatedKeys`))
  (for _index (range (+ (`self.NumVerticalArea`) 1))
    (for _index_2 (range (+ (`self.NumHorizontalArea`) 1))
      (`KismetArrayLibrary.Array_Add` (`self.ActivatedKeys`) (+ (* _index (`self.NumHorizontalArea`)) _index_2)))))

(fn `ActivateAreas`
  (params (PlayerLocationKey :type Integer))
  (locals (locationKey :type Integer))
  (set `local.locationKey` PlayerLocationKey)
  (`KismetArrayLibrary.Array_Clear` (`self.ActivatedKeys`))
  (bind _resultkeys (`self.GetKeysAroundKey` (`local.locationKey`)))
  (set `self.ActivatedKeys` _resultkeys))

(fn `AttachCharacterColliderToAllSnowActors`
  (bind _astest_character_bp (cast `/Game/BP/TestCollisionSampling/TestCharacterBP` (`GameplayStatics.GetPlayerCharacter` 0)))
  (`/Game/BP/TestCollisionSampling/TestCharacterBP.AttachColliders` _astest_character_bp)
  (bind _shovel (`/Game/BP/TestCollisionSampling/TestCharacterBP.Shovel` _astest_character_bp))
  (`/Engine/EditorBlueprintResources/StandardMacros.IsValid` _shovel
    (:`Is Valid`
      (bind _asshovel_bp (cast `/Game/BP/TestCollisionSampling/ShovelBP` (`ChildActorComponent.ChildActor` _shovel)))
      (`/Game/BP/TestCollisionSampling/ShovelBP.AttachColliders` _asshovel_bp)
      (for _array_element (`self.m_snowActors`)
        (`/Game/BP/TestCollisionSampling/TestCharacterBP.UpdatePosition` _astest_character_bp _array_element)))))

(fn `DeleteMesh`
  (params (key :type Integer))
  (`ProceduralMeshComponent.ClearMeshSection` (`self.ProceduralMesh`) key))

(fn `GetKeysAroundKey`
  (params (key :type Integer))
  (returns (resultKeys :type "Array of Integer"))
  (locals (TempKeys :type "Array of Integer"))
  (bind _returnvalue (+ key 1))
  (bind _returnvalue_2 (+ key -1))
  (bind _returnvalue_3 (- key (`self.NumHorizontalArea`)))
  (bind _returnvalue_4 (+ key (`self.NumHorizontalArea`)))
  (bind _returnvalue_5 (+ _returnvalue_4 -1))
  (bind _returnvalue_6 (+ _returnvalue_4 1))
  (bind _returnvalue_7 (+ _returnvalue_3 1))
  (bind _returnvalue_8 (+ _returnvalue_3 -1))
  (`|ExecutionSequence`
    (:`then_0`
      (if (`self.IsValidKey` key)
        (`KismetArrayLibrary.Array_Add` (`local.TempKeys`) key)))
    (:`then_1`
      (if (`self.IsValidKey` _returnvalue)
        (`KismetArrayLibrary.Array_Add` (`local.TempKeys`) _returnvalue)))
    (:`then_2`
      (if (`self.IsValidKey` _returnvalue_2)
        (`KismetArrayLibrary.Array_Add` (`local.TempKeys`) _returnvalue_2)))
    (:`then_3`
      (if (`self.IsValidKey` _returnvalue_3)
        (`KismetArrayLibrary.Array_Add` (`local.TempKeys`) _returnvalue_3)))
    (:`then_4`
      (if (`self.IsValidKey` _returnvalue_7)
        (`KismetArrayLibrary.Array_Add` (`local.TempKeys`) _returnvalue_7)))
    (:`then_5`
      (if (`self.IsValidKey` _returnvalue_8)
        (`KismetArrayLibrary.Array_Add` (`local.TempKeys`) _returnvalue_8)))
    (:`then_6`
      (if (`self.IsValidKey` _returnvalue_4)
        (`KismetArrayLibrary.Array_Add` (`local.TempKeys`) _returnvalue_4)))
    (:`then_7`
      (if (`self.IsValidKey` _returnvalue_6)
        (`KismetArrayLibrary.Array_Add` (`local.TempKeys`) _returnvalue_6)))
    (:`then_8`
      (if (`self.IsValidKey` _returnvalue_5)
        (`KismetArrayLibrary.Array_Add` (`local.TempKeys`) _returnvalue_5)))
    (:`then_9`
      (return (`local.TempKeys`)))))

(fn `InitAreaManager`
  (`self.InitManager` (`SceneComponent.K2_GetComponentLocation` (`self.StartFloor`)) (`SceneComponent.K2_GetComponentLocation` (`self.EndTop`)) (`self.NumHorizontalArea`) (`self.NumVerticalArea`) (`self.NumHorizontalHeightMapElement`) (`self.NumVerticalHeightMapElement`)))

(fn `MakeAreaToHeightMapMesh`
  (params (key :type Integer))
  (if (not (`KismetArrayLibrary.Array_Contains` (`self.HeightMapMeshArea`) key))
    (for _array_element (`self.m_snowActors`)
      (bind _asmy_snow_actor_bp (cast `/Game/BP/MySnowActorBP` _array_element))
      (if (== (`/Game/BP/MySnowActorBP.Key` _asmy_snow_actor_bp) key)
        (`SceneComponent.SetVisibility` (`/Game/BP/MySnowActorBP.InstancedStaticMesh` _asmy_snow_actor_bp) false false)
        (bind _returnvalue (`SnowActorCpp.GetXPos` _array_element))
        (bind _returnvalue_2 (`SnowActorCpp.GetYPos` _array_element))
        (bind _returnvalue_3 (`SnowActorCpp.GetZPos` _array_element))
        (`self.UpdateHeightmap` _returnvalue _returnvalue_2 _returnvalue_3 key)
        (`self.MakeMesh` key)
        (`KismetArrayLibrary.Array_Add` (`self.HeightMapMeshArea`) key)))))

(fn `MakeAreaToParticle`
  (params (Key :type Integer))
  (if (`KismetArrayLibrary.Array_Contains` (`self.HeightMapMeshArea`) Key)
    (for _array_element (`self.m_snowActors`)
      (bind _asmy_snow_actor_bp (cast `/Game/BP/MySnowActorBP` _array_element))
      (if (== (`/Game/BP/MySnowActorBP.Key` _asmy_snow_actor_bp) Key)
        (`SceneComponent.SetVisibility` (`/Game/BP/MySnowActorBP.InstancedStaticMesh` _asmy_snow_actor_bp) true false)
        (`self.DeleteMesh` Key)
        (`KismetArrayLibrary.Array_RemoveItem` (`self.HeightMapMeshArea`) Key)))))

(fn `MakeMesh`
  (params (key :type Integer))
  (bind _returnvalue (`self.GetVertices` key))
  (bind _returnvalue_2 (`self.GetIndices`))
  (`ProceduralMeshComponent.CreateMeshSection_LinearColor` :`self` (`self.ProceduralMesh`) :`SectionIndex` key :`Vertices` _returnvalue :`Triangles` _returnvalue_2)
  (`PrimitiveComponent.SetMaterial` (`self.ProceduralMesh`) key "/Game/CustomMaterial/SnowMaterial_1.SnowMaterial_1"))

(fn `SpawnSnowActor`
  (params (VerticalI :type Integer) (HorizonJ :type Integer))
  (locals (ZOffset :type "Float (double-precision)" :default 40.0))
  (bind _result (`self.MakeSnowActorLocation` VerticalI HorizonJ (`self.m_oneAreaWidth`) (`self.m_oneAreaLength`) (`SceneComponent.K2_GetComponentLocation` (`self.StartFloor`))))
  (bind (_snowactorstartfloor _snowactorendfloor) (`self.MakeSnowActorStartEndFloor` _result (`self.m_oneAreaWidth`) (`self.m_oneAreaLength`) (`self.m_height`)))
  (bind _returnvalue (`|SpawnActorFromClass` "/Game/BP/MySnowActorBP.MySnowActorBP_C" (`KismetMathLibrary.MakeTransform` (+ _result (`KismetMathLibrary.MakeVector` 0.0 0.0 (`local.ZOffset`)))) "Undefined" "OverrideRootScale" null null))
  (`/Game/BP/MySnowActorBP.InitSnowActorBP` _returnvalue _snowactorstartfloor _snowactorendfloor (+ (* VerticalI (`self.NumVerticalArea`)) HorizonJ))
  (`KismetArrayLibrary.Array_Add` (`self.m_snowActors`) _returnvalue))

(fn `UserConstructionScript`
  (bind (_returnvalue_x _returnvalue_y _returnvalue_z) (`KismetMathLibrary.BreakVector` (`SceneComponent.K2_GetComponentLocation` (`self.StartFloor`))))
  (`SceneComponent.SetWorldScale3D` (`self.Box`) (`self.SimArea`))
  (`SceneComponent.K2_SetWorldLocation` (`self.ProceduralMesh`) (`KismetMathLibrary.MakeVector` 0.0 0.0 _returnvalue_z) false false))