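; Shovel test actor that approximates its capsule and two box shapes with sampled sphere colliders.
; BeginPlay sets the CollisionSamplingManager default radius.
; AttachColliders samples each shape through the manager, spawning a BaseColliderActor per sample with its radius and attaching it to that shape, keeping world transform.
; Debug replaces earlier TestSphere markers with new ones at every BaseColliderActor in the world and prints the count.
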(event `self.ReceiveBeginPlay`
  (set `CollisionSamplingManager.defaultRadius` 8.0 (`self.CollisionSamplingManager`)))

(event `self.ReceiveTick`
  (params (DeltaSeconds :type "Float (single-precision)")))

(fn `AttachCollider`
  (params (NewParam :type "ShapeComponent Object Reference"))
  (locals (TempColliderActor :type "BaseColliderActor Object Reference"))
  (bind _collisionsamplingmanager (`self.CollisionSamplingManager`))
  (`CollisionSamplingManager.CollisionSampling` _collisionsamplingmanager (`|MakeArray` NewParam :!type "PrimitiveComponent Object Reference"))
  (for _array_element (`CollisionSamplingManager.ColliderArr` _collisionsamplingmanager)
    (bind (_radius _position) (break `ColliderInfo` _array_element))
    (bind _returnvalue (`|SpawnActorFromClass` "/Script/RealTimeSnowUE.BaseColliderActor" (`KismetMathLibrary.Conv_VectorToTransform` _position) "Undefined" "OverrideRootScale" null null))
    (bind _output_get (set `local.TempColliderActor` _returnvalue))
    (set `BaseColliderActor.radius` _radius _output_get)
    (`self.K2_AttachToComponent` (`local.TempColliderActor`) NewParam "None" "KeepWorld" "KeepWorld" "KeepWorld" false)))

(fn `AttachColliders`
  (bind _output_get (set `self.ColliderArr` (`|MakeArray` (`self.Capsule`) (`self.Box`) (`self.Box1`) :!type "ShapeComponent Object Reference")))
  (for _array_element _output_get
    (`self.AttachCollider` _array_element)))

(fn `Debug`
  (for _array_element (`self.DebugArr`)
    (`self.K2_DestroyActor` _array_element))
  (`KismetArrayLibrary.Array_Clear` (`self.DebugArr`))
  (bind _outactors (`GameplayStatics.GetAllActorsOfClass` "/Script/RealTimeSnowUE.BaseColliderActor"))
  (for _array_element_2 _outactors
    (bind _returnvalue (`|SpawnActorFromClass` "/Game/BP/TestCollisionSampling/TestSphere.TestSphere_C" (`KismetMathLibrary.Conv_VectorToTransform` (`self.K2_GetActorLocation` _array_element_2)) "Undefined" "OverrideRootScale" null (`BaseColliderActor.radius` _array_element_2) null))
    (`KismetArrayLibrary.Array_Add` (`self.DebugArr`) _returnvalue))
  (`KismetSystemLibrary.PrintString` (`KismetStringLibrary.Conv_IntToString` (`KismetArrayLibrary.Array_Length` _outactors))))

(fn `UserConstructionScript`)