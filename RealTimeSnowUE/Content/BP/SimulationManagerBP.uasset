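; Manager Blueprint that runs a particle-based snow simulation across keyed areas and handles its input.
; While simulating, Tick has SnowAreaManager turn activated areas into particles and the rest into heightmap meshes as a level of detail, simulating only the player's area.
; DoSimulation toggles the manager and activated snow actors, setting physical parameters on those it starts.
; Other inputs toggle help and parameter widgets; a camera-trace function highlights a debug particle.
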(event `self.ReceiveBeginPlay`
  ;[1 1 1] 초기화
  (`self.EnableInput` (`GameplayStatics.GetPlayerController` 0)))

(event `self.ReceiveTick`
  (params (DeltaSeconds :type "Float (single-precision)"))
  ;[1 1 1] Event Tick
  (if (`self.isSimulating`)
    (`self.ActivateDeactivateSnowActors` (`/Game/BP/SnowAreaManagerBP.ActivatedKeys` (`self.SnowAreaManager`)))))

(event `InputAction|DoSimulation`
  (params (Key :type "Key Structure"))
  ;[1 1 1] 시작/재개/일시정지
  (:`Pressed`
    (set `self.isSimulating` (not (`self.isSimulating`)))
    (bind _newparam (`self.GetActivatedSnowActors`))
    (for _array_element _newparam
      (bind _asmy_snow_actor_bp (cast `/Game/BP/MySnowActorBP` _array_element))
      (if (`/Game/BP/MySnowActorBP.IsSimulating` _asmy_snow_actor_bp)
        (set `/Game/BP/MySnowActorBP.IsSimulating` false _asmy_snow_actor_bp)
        (else
          (`SnowActorCpp.SetParams` _asmy_snow_actor_bp 0.0125 5.0 5000.0 25000.0 0.05 0.025)
          (set `/Game/BP/MySnowActorBP.IsSimulating` true _asmy_snow_actor_bp))))))

(event `InputAction|HowUIOnOff`
  (params (Key :type "Key Structure"))
  (bind _howtoplaywidget (`self.HowToPlayWidget`))
  ;[1 1 1] ui on/off
  (:`Pressed`
    (`/Engine/EditorBlueprintResources/StandardMacros.FlipFlop`
      (:`A`
        (`Widget.SetVisibility` _howtoplaywidget "Hidden"))
      (:`B`
        (`Widget.SetVisibility` _howtoplaywidget "Visible")))))

(event `InputAction|ParamUIOnOff`
  (params (Key :type "Key Structure"))
  (bind _paramwidget (`self.ParamWidget`))
  ;[1 1 1] ui on/off
  (:`Pressed`
    (`/Engine/EditorBlueprintResources/StandardMacros.FlipFlop`
      (:`A`
        (`Widget.SetVisibility` _paramwidget "Hidden"))
      (:`B`
        (`Widget.SetVisibility` _paramwidget "Visible")))))

(event `InputAction|MoveColliderForward`
  (params (Key :type "Key Structure"))
  ;[1 1 1] set collider velocity
)

(event `InputAction|MoveColliderUp`
  (params (Key :type "Key Structure"))
  ;[1 1 1] set collider velocity
)

(event `InputAction|MoveColliderBack`
  (params (Key :type "Key Structure"))
  ;[1 1 1] set collider velocity
)

(event `InputAction|MoveColliderDown`
  (params (Key :type "Key Structure"))
  ;[1 1 1] set collider velocity
)

(event `InputAction|MoveColliderLeft`
  (params (Key :type "Key Structure"))
  ;[1 1 1] set collider velocity
)

(event `InputAction|MoveColliderRight`
  (params (Key :type "Key Structure"))
  ;[1 1 1] set collider velocity
)

(fn `ActivateDeactivateSnowActors`
  (params (ActivatedKeys :type "Array of Integer"))
  (bind _snowareamanager (`self.SnowAreaManager`))
  (for _array_element (`SnowAreaManager.m_snowActors` (`self.SnowAreaManager`))
    (bind _asmy_snow_actor_bp (cast `/Game/BP/MySnowActorBP` _array_element))
    (bind _key (`/Game/BP/MySnowActorBP.Key` _asmy_snow_actor_bp))
    (if (`KismetArrayLibrary.Array_Contains` ActivatedKeys _key)
      (`/Game/BP/SnowAreaManagerBP.MakeAreaToParticle` _snowareamanager _key)
      (bind _returnvalue (`SnowAreaManager.GetAreaKey` (`self.SnowAreaManager`) (`self.K2_GetActorLocation` (`GameplayStatics.GetPlayerCharacter` 0))))
      (if (== _returnvalue _key)
        (set `/Game/BP/MySnowActorBP.IsSimulating` true _asmy_snow_actor_bp)
        (else
          (set `/Game/BP/MySnowActorBP.IsSimulating` false _asmy_snow_actor_bp)))
      (else
        (`/Game/BP/SnowAreaManagerBP.MakeAreaToHeightMapMesh` _snowareamanager _key)))))

(fn `Debug_LineTraceToParticle`
  (bind _debuggingparticle (`self.DebuggingParticle`))
  (bind _returnvalue (`self.K2_GetActorLocation` (`GameplayStatics.GetPlayerPawn` 0)))
  ;[1 1 1] 플레이어 화면->particle로 광선을 쏴서 디버깅 대상 파티클로 지정
  (bind _outhit (`KismetSystemLibrary.LineTraceSingle` :`Start` _returnvalue :`End` (+ _returnvalue (* (`self.GetActorForwardVector` (`GameplayStatics.GetPlayerCameraManager` 0)) 1000.0)) :`TraceChannel` "TraceTypeQuery1" :`DrawDebugType` "ForOneFrame"))
  (bind _asmy_snow_paritcle_bp (cast `/Game/BP/MySnowParitcleBP` (`.HitActor` (`GameplayStatics.BreakHitResult` _outhit))))
  (`/Engine/EditorBlueprintResources/StandardMacros.IsValid` _debuggingparticle
    (:`Is Valid`
      (`PrimitiveComponent.SetMaterial` (`/Game/BP/MySnowParitcleBP.Cube` _debuggingparticle) 0 "/Engine/BasicShapes/BasicShapeMaterial.BasicShapeMaterial"))
    (:`Is Not Valid`
      _))
  (bind _output_get (set `self.DebuggingParticle` _asmy_snow_paritcle_bp))
  (`PrimitiveComponent.SetMaterial` (`/Game/BP/MySnowParitcleBP.Cube` _output_get) 0 "/Game/CustomMaterial/VeryBrightMaterial.VeryBrightMaterial"))

(fn `GetActivatedSnowActors`
  (returns (NewParam :type "Array of /Game/BP/MySnowActorBP Object Reference"))
  (locals (SnowActors :type "Array of /Game/BP/MySnowActorBP Object Reference"))
  (bind _snowareamanager (`self.SnowAreaManager`))
  (bind _returnvalue (`SnowAreaManager.GetSnowActors` _snowareamanager))
  (for _array_element _returnvalue
    (bind _asmy_snow_actor_bp (cast `/Game/BP/MySnowActorBP` _array_element))
    (if (`KismetArrayLibrary.Array_Contains` (`/Game/BP/SnowAreaManagerBP.ActivatedKeys` _snowareamanager) (`/Game/BP/MySnowActorBP.Key` _asmy_snow_actor_bp))
      (`KismetArrayLibrary.Array_Add` (`local.SnowActors`) _asmy_snow_actor_bp)))
  (return (`local.SnowActors`)))

(fn `UserConstructionScript`)